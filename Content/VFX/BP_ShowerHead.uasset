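; BP_ShowerHead is a VFX actor that drives a Niagara water spray effect for a shower head.
; Its Construction Script copies exposed variables for fall height, pressure, spray shape, speed, drop look and water material into the Niagara component's user parameters.
; An Enabled variable sets whether the effect auto-activates.
; The event graph holds only disabled placeholder events, so the Blueprint adds no runtime logic.
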(event EventBeginPlay)

(event Collision|EventActorBeginOverlap
  (params (OtherActor :type Actor%20Object%20Reference)))

(event EventTick
  (params (DeltaSeconds :type Float%20%28single-precision%29)))

(fn ConstructionScript
  (bind _niagara (Variables|Default|GetNiagara))
  (Niagara|SetNiagaraVariable(Float) _niagara "User.FallHeight" (Variables|Shower|GetUser.FallHeight))
  (Niagara|SetNiagaraVariable(Float) _niagara "User.Pressure" (Variables|Shower|GetUser.Pressure))
  (Niagara|SetNiagaraVariable(Float) _niagara "User.SprayAngle" (Variables|Shower|GetUser.SprayAngle))
  (Niagara|SetNiagaraVariable(Float) _niagara "User.SprayRadius" (Variables|Shower|GetUser.SprayRadius))
  (Niagara|SetNiagaraVariable(Float) _niagara "User.Speed" (Variables|Shower|GetSpeed))
  (Niagara|SetNiagaraVariable(Float) _niagara "User.DropIntensity" (Variables|Shower|GetDropIntensity))
  (Niagara|SetNiagaraVariable(Float) _niagara "User.DropSize" (Variables|Shower|GetDropSize))
  (Class|NiagaraComponent|SetVariableMaterial _niagara "User.WaterMaterial" (Variables|Shower|GetWaterMaterial))
  (Components|Activation|SetAutoActivate _niagara (Variables|Shower|GetEnabled)))